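; PC_MP is a multiplayer player controller that lets a player without a pawn request a respawn.
; Pressing P checks that no valid pawn is controlled, then calls the server respawn request event.
; That event casts the game mode to MP_GM and passes this controller to its ServerRespawnPlayer, leaving the respawn itself to the game mode.
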(event Custom|Server_RequestRespawn
  (bind _returnvalue (Game|GetGameMode))
  ;[1 1 1] Respawn Player Calls Custom Event In Game Mode
  (Utilities|IsValid _returnvalue
    (:Is%20Valid
      (bind _asmp_gm (Utilities|Casting|CastToMP_GM _returnvalue))
      (Utilities|IsValid _asmp_gm
        (:Is%20Valid
          (Default|ServerRespawnPlayer _asmp_gm self))))))

(event Input|KeyboardEvents|P
  (params (Key :type Key%20Structure))
  ;[1 1 1] Respawn Player Calls Custom Event In Game Mode
  (:Pressed
    (Utilities|IsValid (Pawn|GetControlledPawn self)
      (:Is%20Not%20Valid
        (CallFunction|ServerRequestRespawn)))))

(fn ConstructionScript)